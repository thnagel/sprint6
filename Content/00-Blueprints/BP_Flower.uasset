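; BP_Flower is an actor with an animated Arrow component that spins and floats up and down.
; On BeginPlay it creates its own WBP_HUD, adds it to the viewport with the info text hidden, and caches the arrow's starting height.
; Each Tick it rolls the arrow at a frame-rate independent speed and bobs it around that height with a sine of game time.
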(event EventBeginPlay
  (bind _returnvalue (UserInterface|CreateWidget "/Game/00-Blueprints/Widgets/WBP_HUD.WBP_HUD_C"))
  (Variables|Default|SetHUDRef _returnvalue)
  (UserInterface|Viewport|AddtoViewport (Variables|Default|GetHUDRef) 0)
  (Default|HideInfoText (Variables|Default|GetHUDRef))
  (Variables|Default|SetOriginHeight (.z (.location (Transformation|GetRelativeTransform (Variables|Default|GetArrow))))))

(event EventTick
  (params (DeltaSeconds :type Float%20%28single-precision%29))
  (Transformation|AddLocalRotation (Variables|Default|GetArrow) (Math|Rotator|MakeRotator (* (Variables|Default|GetRotationSpeed) DeltaSeconds) 0.0 0.0) false false)
  (Transformation|SetRelativeLocation (Variables|Default|GetArrow) (Math|Vector|MakeVector 0.0 0.0 (+ (* (Math|Trig|Sin(Radians) (* (Utilities|Time|GetGameTimeinSeconds) (Variables|Default|GetFloatingSpeed))) (Variables|Default|GetFloatingHeight)) (Variables|Default|GetOriginHeight))) false false))

(fn ConstructionScript)